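; Actor component that records a participant session to files, apparently for an experiment, starting on BeginPlay and saving on EndPlay.
; A looping timer samples owner position, control rotation, speed and FPS into a stream buffer, while LogEvent appends named, positioned events to a second buffer.
; EndSession writes both buffers as CSV plus a metadata JSON with condition and movement settings, all named by session ID.
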(event `StartSession`
  (if (`self.bIsLogging`)
    (`KismetSystemLibrary.PrintString` "ATTENZIONE: StartSession chiamato due volte")
    (else
      (set `self.bIsLogging` true)
      (`KismetArrayLibrary.Array_Clear` (`self.StreamRows`))
      (`KismetArrayLibrary.Array_Clear` (`self.EventRows`))
      (set `self.SessionStartTime` (`KismetSystemLibrary.GetGameTimeInSeconds`))
      (bind _returnvalue (`CoppitoTwinFileLibrary.MakeSessionId` (`self.ParticipantID`)))
      (set `self.SessionID` _returnvalue)
      (`KismetArrayLibrary.Array_Add` (`self.StreamRows`) "t,pos_x,pos_y,pos_z,cam_yaw,cam_pitch,speed,fps")
      (`KismetArrayLibrary.Array_Add` (`self.EventRows`) "t,event,value,pos_x,pos_y,pos_z")
      (bind _returnvalue_2 (`KismetSystemLibrary.K2_SetTimerDelegate` (delegate `LogSample`) (`self.SampleInterval`) true))
      (set `self.SampleTimer` _returnvalue_2))))

(event `LogSample`
  (bind _returnvalue (`self.GetOwner`))
  (`KismetArrayLibrary.Array_Add` (`self.StreamRows`) (`CoppitoTwinFileLibrary.MakeStreamRow` (- (`KismetSystemLibrary.GetGameTimeInSeconds`) (`self.SessionStartTime`)) (`Actor.K2_GetActorLocation` _returnvalue) (.yaw (`Controller.GetControlRotation` (`GameplayStatics.GetPlayerController` 0))) (.pitch (`Controller.GetControlRotation` (`GameplayStatics.GetPlayerController` 0))) (`KismetMathLibrary.VSize` (`Actor.GetVelocity` _returnvalue)) (/ 1.0 (`GameplayStatics.GetWorldDeltaSeconds`)))))

(event `EndSession`
  (if (`self.bIsLogging`)
    (`KismetSystemLibrary.K2_ClearAndInvalidateTimerHandle` (`self.SampleTimer`))
    (set `self.bIsLogging` false)
    (bind _returnvalue (`CoppitoTwinFileLibrary.SaveLinesToFile` (`self.StreamRows`) (`KismetStringLibrary.Concat_StrStr` (`self.SessionID`) "_stream.csv")))
    (`KismetSystemLibrary.PrintString` (`KismetStringLibrary.Concat_StrStr` "STREAM salvato: " (`KismetStringLibrary.Conv_BoolToString` _returnvalue)) true true (struct :`G` 0.66 :`B` 1.0 :`A` 1.0) 10.0)
    (bind _returnvalue_2 (`CoppitoTwinFileLibrary.SaveLinesToFile` (`self.EventRows`) (`KismetStringLibrary.Concat_StrStr` (`self.SessionID`) "_events.csv")))
    (`KismetSystemLibrary.PrintString` (`KismetStringLibrary.Concat_StrStr` "EVENTI salvato: " (`KismetStringLibrary.Conv_BoolToString` _returnvalue_2)) true true (struct :`G` 0.66 :`B` 1.0 :`A` 1.0) 10.0)
    (`KismetSystemLibrary.PrintString` (`KismetStringLibrary.Concat_StrStr` "campioni raccolti: " (`KismetStringLibrary.Conv_IntToString` (- (`KismetArrayLibrary.Array_Length` (`self.StreamRows`)) 1))) true true (struct :`G` 0.66 :`B` 1.0 :`A` 1.0) 10.0)
    (`CoppitoTwinFileLibrary.SaveSessionMetadata` (`Actor.GetComponentByClass` (`self.GetOwner`) "/Script/Engine.CharacterMovementComponent") (`self.ParticipantID`) (`self.Condition`) (`self.BarruerConfig`) (/ 1.0 (`self.SampleInterval`)) (`self.MinPathCm`) (- (`KismetSystemLibrary.GetGameTimeInSeconds`) (`self.SessionStartTime`)) (- (`KismetArrayLibrary.Array_Length` (`self.StreamRows`)) 1) (- (`KismetArrayLibrary.Array_Length` (`self.EventRows`)) 1) (`KismetStringLibrary.Concat_StrStr` (`self.SessionID`) "_meta.json"))
    (else
      (`KismetSystemLibrary.PrintString` "ATTENZIONE: EndSession senza sessione attiva"))))

(event `self.ReceiveBeginPlay`
  (`self.StartSession`))

(event `LogEvent`
  (params (EventName :type String) (Value :type String))
  (if (`self.bIsLogging`)
    (if (`KismetStringLibrary.NotEqual_StrStr` EventName)
      (`KismetArrayLibrary.Array_Add` (`self.EventRows`) (`CoppitoTwinFileLibrary.MakeEventRow` (- (`KismetSystemLibrary.GetGameTimeInSeconds`) (`self.SessionStartTime`)) EventName Value (`Actor.K2_GetActorLocation` (`self.GetOwner`))))
      (else
        (`KismetSystemLibrary.PrintString` "TRIGGER SENZA NOME" false)))))

(event `self.ReceiveEndPlay`
  (params (EndPlayReason :type "EEndPlayReason Enum" :default "Destroyed"))
  (`self.LogEvent` "SESSION_ABORT" "chiusura")
  (`self.EndSession`))