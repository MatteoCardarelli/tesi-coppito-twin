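; BP_EventTrigger is a placeable box trigger that logs named events when actors enter or leave it.
; On overlap begin, it finds a BP_LoggerComponent on the other actor and calls LogEvent with its EventName and Value.
; On overlap end, it logs EventNameOnExit with the same Value, but only when that name is not empty.
; Actors without a logger component are ignored.
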(event `self.Box.OnComponentBeginOverlap`
  (params (OverlappedComponent :type "PrimitiveComponent Object Reference") (OtherActor :type "Actor Object Reference") (OtherComp :type "PrimitiveComponent Object Reference") (OtherBodyIndex :type Integer) (bFromSweep :type Boolean) (SweepResult :type "HitResult Structure (by ref)"))
  (bind _returnvalue (`self.GetComponentByClass` OtherActor "/Game/Logging/BP_LoggerComponent.BP_LoggerComponent_C"))
  (if (`KismetSystemLibrary.IsValid` _returnvalue)
    (`/Game/Logging/BP_LoggerComponent.LogEvent` _returnvalue (`self.EventName`) (`self.Value`))))

(event `self.Box.OnComponentEndOverlap`
  (params (OverlappedComponent :type "PrimitiveComponent Object Reference") (OtherActor :type "Actor Object Reference") (OtherComp :type "PrimitiveComponent Object Reference") (OtherBodyIndex :type Integer))
  (bind _returnvalue (`self.GetComponentByClass` OtherActor "/Game/Logging/BP_LoggerComponent.BP_LoggerComponent_C"))
  (if (`KismetStringLibrary.NotEqual_StrStr` (`self.EventNameOnExit`))
    (if (`KismetSystemLibrary.IsValid` _returnvalue)
      (`/Game/Logging/BP_LoggerComponent.LogEvent` _returnvalue (`self.EventNameOnExit`) (`self.Value`)))))

(fn `UserConstructionScript`)